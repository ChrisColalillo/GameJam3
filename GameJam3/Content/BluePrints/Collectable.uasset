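; Collectable is a spinning pickup that spawns two extra Ball_Angry actors when touched by an actor tagged "Ball".
; Tick applies a steady local yaw rotation.
; On any overlap it disables the static mesh's collision before checking the tag.
; For a ball, it spawns the pair offset to either side along world Y, then destroys itself after a short delay.
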(event EventTick
  (params (DeltaSeconds :type Float%20%28single-precision%29))
  (Transformation|AddActorLocalRotation (Math|Rotator|MakeRotator 0.0 0.0 0.7) false false))

(event Collision|EventActorBeginOverlap
  (params (OtherActor :type Actor%20Object%20Reference))
  (bind _defaultsceneroot (Variables|Default|GetDefaultSceneRoot))
  (bind _returnvalue (Transformation|GetWorldLocation _defaultsceneroot))
  (Collision|SetCollisionEnabled (Variables|Default|GetStaticMesh) "NoCollision")
  (if (Actor|ActorHasTag OtherActor "Ball")
    (Game|SpawnActorfromClass "/Game/BluePrints/Ball_Angry.Ball_Angry_C" (Math|Transform|MakeTransform (Math|Vector|MakeVector (.x _returnvalue) (+ (.y _returnvalue) 8e+01) (.z _returnvalue)) "0, 0, 0" "1,1,1") "AdjustIfPossibleButAlwaysSpawn" 0 0)
    (Game|SpawnActorfromClass "/Game/BluePrints/Ball_Angry.Ball_Angry_C" (Math|Transform|MakeTransform (Math|Vector|MakeVector (.x _returnvalue) (+ (.y _returnvalue) -8e+01) (.z _returnvalue)) "0, 0, 0" "1,1,1") "AdjustIfPossibleButAlwaysSpawn" 0 0)
    (Utilities|FlowControl|Delay 0.1)
    (Actor|DestroyActor)))

(fn ConstructionScript)