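; Player camera Blueprint that tilts and turns the Box actor from axis input and can freeze all Ball_Ryan actors.
; Box rotations use axes from the camera's yaw, and SwitchLeft/SwitchRight cycle the camera through four hard-coded side views.
; Holding Jump stops ball physics and makes the Box root Static; release restores both.
; A Tick-driven Delay counts down the freeze cooldown only while move input is non-zero.
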(event EventTick
  (params (DeltaSeconds :type Float%20%28single-precision%29))
  ;[1 1 1] Freeze Cooldown
  (if (and (or (!= (Variables|Default|GetisRotatingx) 0.0) (!= (Variables|Default|GetisRotatingy) 0.0)) (Variables|Default|GetOnCooldown))
    (Utilities|FlowControl|Delay 1.0)
    (bind _output_get (Variables|Default|SetCooldown (+ (Variables|Default|GetCooldown) 1)))
    (Development|PrintString (Utilities|String|ToString(Integer) _output_get) true true "(R=0.000000,G=0.015310,B=0.432292,A=1.000000)")
    (if (>= (Variables|Default|GetCooldown) 5)
      (Variables|Default|SetOnCooldown false)
      (Variables|Default|SetCooldown 0))))

(event EventBeginPlay
  ;[1 1 1] Cube Rotation
  (bind _returnvalue (Actor|GetActorOfClass "/Game/BluePrints/Box.Box_C")))

(event Input|ActionEvents|InputActionSwitchLeft
  (params (Key :type Key%20Structure :default "None"))
  (bind _camera (Variables|Default|GetCamera))
  ;[1 1 1] Scuffed Camera Rotation
  (:Pressed
    (if (== (Variables|Default|GetCameraNumber) 0)
      (Transformation|SetWorldLocationAndRotation _camera "0.000000,-4000.000000,1280.000000" "-20.000000,90.000000, 0" false false)
      (Variables|Default|SetCameraNumber 1)
      (elif (== (Variables|Default|GetCameraNumber) 1)
        (Transformation|SetWorldLocationAndRotation _camera "4000.000000,0.000000,1280.000000" "-20.000000,180.000000, 0" false false)
        (Variables|Default|SetCameraNumber 2)
        (elif (== (Variables|Default|GetCameraNumber) 2)
          (Transformation|SetWorldLocationAndRotation _camera "0.000000,4000.000000,1280.000000" "-20.000000,-90.000000, 0" false false)
          (Variables|Default|SetCameraNumber 3)
          (elif (== (Variables|Default|GetCameraNumber) 3)
            (Transformation|SetWorldLocationAndRotation _camera "-4000.000000,0.000000,1280.000000" "-20.000000,0.000000, 0" false false)
            (Variables|Default|SetCameraNumber 0)))))))

(event Input|ActionEvents|InputActionSwitchRight
  (params (Key :type Key%20Structure :default "None"))
  (bind _camera (Variables|Default|GetCamera))
  ;[1 1 1] Scuffed Camera Rotation
  (:Pressed
    (if (== (Variables|Default|GetCameraNumber) 2)
      (Transformation|SetWorldLocationAndRotation _camera "0.000000,-4000.000000,1280.000000" "-20.000000,90.000000, 0" false false)
      (Variables|Default|SetCameraNumber 1)
      (elif (== (Variables|Default|GetCameraNumber) 3)
        (Transformation|SetWorldLocationAndRotation _camera "4000.000000,0.000000,1280.000000" "-20.000000,180.000000, 0" false false)
        (Variables|Default|SetCameraNumber 2)
        (elif (== (Variables|Default|GetCameraNumber) 0)
          (Transformation|SetWorldLocationAndRotation _camera "0.000000,4000.000000,1280.000000" "-20.000000,-90.000000, 0" false false)
          (Variables|Default|SetCameraNumber 3)
          (elif (== (Variables|Default|GetCameraNumber) 1)
            (Transformation|SetWorldLocationAndRotation _camera "-4000.000000,0.000000,1280.000000" "-20.000000,0.000000, 0" false false)
            (Variables|Default|SetCameraNumber 0)))))))

(event Input|ActionEvents|InputActionJump
  (params (Key :type Key%20Structure :default "None"))
  ;[1 1 1] Scuffed Freeze All Balls
  (:Pressed
    (if (not (Variables|Default|GetOnCooldown))
      (bind _outactors (Actor|GetAllActorsOfClass "/Game/BluePrints/Ball_Ryan.Ball_Ryan_C"))
      (for _array_element _outactors
        (if (Variables|/Game/BluePrints/Ball_Ryan.Ball_Ryan_C|GetPhysics _array_element)
          (Physics|SetSimulatePhysics (Variables|/Game/BluePrints/Ball_Ryan.Ball_Ryan_C|GetSphere _array_element) false)
          (Variables|/Game/BluePrints/Ball_Ryan.Ball_Ryan_C|SetPhysics _array_element false)
          (Variables|Default|SetCooldown 0)
          (Variables|Default|SetOnCooldown true)))
      (bind _returnvalue (Actor|GetActorOfClass "/Game/BluePrints/Box.Box_C"))
      (Transformation|SetMobility (Variables|/Game/BluePrints/Box.Box_C|GetDefaultSceneRoot _returnvalue) "Static")))
  (:Released
    (bind _outactors_2 (Actor|GetAllActorsOfClass "/Game/BluePrints/Ball_Ryan.Ball_Ryan_C"))
    (for _array_element_2 _outactors_2
      (if (not (Variables|/Game/BluePrints/Ball_Ryan.Ball_Ryan_C|GetPhysics _array_element_2))
        (Physics|SetSimulatePhysics (Variables|/Game/BluePrints/Ball_Ryan.Ball_Ryan_C|GetSphere _array_element_2) true)
        (Variables|/Game/BluePrints/Ball_Ryan.Ball_Ryan_C|SetPhysics _array_element_2 true)))
    (bind _returnvalue_2 (Actor|GetActorOfClass "/Game/BluePrints/Box.Box_C"))
    (Transformation|SetMobility (Variables|/Game/BluePrints/Box.Box_C|GetDefaultSceneRoot _returnvalue_2) "Movable")))

(event Input|AxisEvents|InputAxisMoveForward
  (params (AxisValue :type Float%20%28single-precision%29))
  (bind _camera (Variables|Default|GetCamera))
  ;[1 1 1] Cube Rotation
  (bind _output_get (Variables|Default|SetisRotatingy (* AxisValue (Variables|Default|GetBaseLookUpRate) (Utilities|Time|GetWorldDeltaSeconds))))
  (Class|Actor|AddActorWorldRotation (stale EventBeginPlay _returnvalue) (Math|Rotator|CombineRotators (Math|Vector|RotatorfromAxisandAngle (Math|Vector|GetForwardVector (Math|Rotator|MakeRotator 0.0 0.0 (.Yaw (Math|Rotator|BreakRotator (Transformation|GetWorldRotation _camera))))) (stale Input|AxisEvents|InputAxisMoveRight _output_get)) (Math|Vector|RotatorfromAxisandAngle (Math|Vector|GetRightVector (Math|Rotator|MakeRotator 0.0 0.0 (.Yaw (Math|Rotator|BreakRotator (Transformation|GetWorldRotation _camera))))) _output_get))))

(event Input|AxisEvents|InputAxisMoveRight
  (params (AxisValue :type Float%20%28single-precision%29))
  (bind _camera (Variables|Default|GetCamera))
  ;[1 1 1] Cube Rotation
  (bind _output_get (Variables|Default|SetisRotatingx (* AxisValue (Variables|Default|GetBaseTurnRate) (Utilities|Time|GetWorldDeltaSeconds))))
  (Class|Actor|AddActorWorldRotation (stale EventBeginPlay _returnvalue) (Math|Rotator|CombineRotators (Math|Vector|RotatorfromAxisandAngle (Math|Vector|GetForwardVector (Math|Rotator|MakeRotator 0.0 0.0 (.Yaw (Math|Rotator|BreakRotator (Transformation|GetWorldRotation _camera))))) _output_get) (Math|Vector|RotatorfromAxisandAngle (Math|Vector|GetRightVector (Math|Rotator|MakeRotator 0.0 0.0 (.Yaw (Math|Rotator|BreakRotator (Transformation|GetWorldRotation _camera))))) (stale Input|AxisEvents|InputAxisMoveForward _output_get)))))

(event Input|AxisEvents|InputAxisTurnRate
  (params (AxisValue :type Float%20%28single-precision%29))
  (bind _output_get (Variables|Default|SetisRotatingz (* AxisValue (Variables|Default|GetBaseTurnRate) (Utilities|Time|GetWorldDeltaSeconds))))
  (Class|Actor|AddActorWorldRotation (stale EventBeginPlay _returnvalue) (Math|Vector|RotatorfromAxisandAngle (Math|Vector|GetUpVector (Math|Rotator|MakeRotator 0.0 0.0 (.Yaw (Math|Rotator|BreakRotator (Transformation|GetWorldRotation (Variables|Default|GetCamera)))))) _output_get)))

(fn ConstructionScript)