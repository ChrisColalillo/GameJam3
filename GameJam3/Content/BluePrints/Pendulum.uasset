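; Pendulum actor that swings a mesh and scores tagged balls that overlap it.
; On BeginPlay, the PendulumSwing timeline drives the pitch of StaticMesh1.
; Overlapping actors tagged Ball raise the CameraPlayer's Score by one if also tagged Red, otherwise lower it by one.
; The new score prints on screen in green or red, and the ball is destroyed.
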(event EventBeginPlay
  (bind _pendulumswing (Timeline|PendulumSwing Play)
    (:Update
      (Transformation|SetRelativeLocationAndRotation (Variables|Default|GetStaticMesh1) "0, 0, 0" (Math|Rotator|MakeRotator 0.0 (.y _pendulumswing) 0.0) false false))))

(event Collision|EventActorBeginOverlap
  (params (OtherActor :type Actor%20Object%20Reference))
  (if (Actor|ActorHasTag OtherActor "Ball")
    (if (Actor|ActorHasTag OtherActor "Red")
      (bind _returnvalue (Actor|GetActorOfClass "/Game/BluePrints/CameraPlayer.CameraPlayer_C"))
      (bind _output_get (Variables|/Game/BluePrints/CameraPlayer.CameraPlayer_C|SetScore _returnvalue (+ (Variables|/Game/BluePrints/CameraPlayer.CameraPlayer_C|GetScore _returnvalue) 1)))
      (Development|PrintString (Utilities|String|ToString(Integer) _output_get) true true "(R=0.000000,G=0.421875,B=0.030447,A=1.000000)")
      (else
        (bind _returnvalue_2 (Actor|GetActorOfClass "/Game/BluePrints/CameraPlayer.CameraPlayer_C"))
        (bind _output_get_2 (Variables|/Game/BluePrints/CameraPlayer.CameraPlayer_C|SetScore _returnvalue_2 (+ (Variables|/Game/BluePrints/CameraPlayer.CameraPlayer_C|GetScore _returnvalue_2) -1)))
        (Development|PrintString (Utilities|String|ToString(Integer) _output_get_2) true true "(R=0.427083,G=0.000000,B=0.010946,A=1.000000)")))
    (Actor|DestroyActor OtherActor)))

(fn ConstructionScript)