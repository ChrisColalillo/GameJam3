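; Pressure plate that switches laser beams and their collision when an actor tagged Ball overlaps its box.
; On BeginPlay it derives its plate number from the sign of its world Y and Z position, so behavior depends on level placement.
; Plate 1 turns on the Laser actor's beam for two seconds, while plates 2 and 3 turn Laser2's beam on and off respectively, finding each laser by class.
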(event OnComponentBeginOverlap(Box)
  (params (OverlappedComponent :type Primitive%20Component%20Object%20Reference) (OtherActor :type Actor%20Object%20Reference) (OtherComp :type Primitive%20Component%20Object%20Reference) (OtherBodyIndex :type Integer) (bFromSweep :type Boolean) (SweepResult :type Hit%20Result%20Structure%20%28by%20ref%29))
  (if (Actor|ActorHasTag OtherActor "Ball")
    (if (== (Variables|Default|GetPlate%20number) 1)
      (bind _returnvalue (Actor|GetActorOfClass "/Game/BluePrints/Laser.Laser_C"))
      (Rendering|SetVisibility (Variables|/Game/BluePrints/Laser.Laser_C|GetLazer1 _returnvalue) true false)
      (Collision|SetCollisionEnabled (Variables|/Game/BluePrints/Laser.Laser_C|GetLazer1 _returnvalue) "QueryOnly")
      (Utilities|FlowControl|Delay 2.0)
      (Rendering|SetVisibility (Variables|/Game/BluePrints/Laser.Laser_C|GetLazer1 _returnvalue) false false)
      (Collision|SetCollisionEnabled (Variables|/Game/BluePrints/Laser.Laser_C|GetLazer1 _returnvalue) "NoCollision")
      (elif (== (Variables|Default|GetPlate%20number) 2)
        (bind _returnvalue_2 (Actor|GetActorOfClass "/Game/BluePrints/Laser2.Laser2_C"))
        (Rendering|SetVisibility (Variables|/Game/BluePrints/Laser2.Laser2_C|GetLazer1 _returnvalue_2) true false)
        (Collision|SetCollisionEnabled (Variables|/Game/BluePrints/Laser2.Laser2_C|GetLazer1 _returnvalue_2) "QueryOnly")
        (elif (== (Variables|Default|GetPlate%20number) 3)
          (bind _returnvalue_3 (Actor|GetActorOfClass "/Game/BluePrints/Laser2.Laser2_C"))
          (Rendering|SetVisibility (Variables|/Game/BluePrints/Laser2.Laser2_C|GetLazer1 _returnvalue_3) false false)
          (Collision|SetCollisionEnabled (Variables|/Game/BluePrints/Laser2.Laser2_C|GetLazer1 _returnvalue_3) "NoCollision"))))))

(event EventBeginPlay
  (bind _defaultsceneroot (Variables|Default|GetDefaultSceneRoot))
  (bind _returnvalue (Transformation|GetWorldLocation _defaultsceneroot))
  (if (> (.y _returnvalue) 0.0)
    (Variables|Default|SetPlate%20number 2)
    (elif (< (.z _returnvalue) 0.0)
      (Variables|Default|SetPlate%20number 3)
      (else
        (Variables|Default|SetPlate%20number 1)))))

(fn ConstructionScript)