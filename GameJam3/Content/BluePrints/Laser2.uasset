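; Laser2 is a Blueprint laser zone that scores balls by color when they touch it and removes them from play.
; On overlap with its Lazer1 component, an actor tagged Ball adds a point to the CameraPlayer's Score if also tagged Red, otherwise subtracts one.
; The new score prints on screen in green or red, then the ball is destroyed.
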(event OnComponentBeginOverlap(Lazer1)
  (params (OverlappedComponent :type Primitive%20Component%20Object%20Reference) (OtherActor :type Actor%20Object%20Reference) (OtherComp :type Primitive%20Component%20Object%20Reference) (OtherBodyIndex :type Integer) (bFromSweep :type Boolean) (SweepResult :type Hit%20Result%20Structure%20%28by%20ref%29))
  (if (Actor|ActorHasTag OtherActor "Ball")
    (if (Actor|ActorHasTag OtherActor "Red")
      (bind _returnvalue (Actor|GetActorOfClass "/Game/BluePrints/CameraPlayer.CameraPlayer_C"))
      (bind _output_get (Variables|/Game/BluePrints/CameraPlayer.CameraPlayer_C|SetScore _returnvalue (+ (Variables|/Game/BluePrints/CameraPlayer.CameraPlayer_C|GetScore _returnvalue) 1)))
      (Development|PrintString (Utilities|String|ToString(Integer) _output_get) true true "(R=0.000000,G=0.421875,B=0.030447,A=1.000000)")
      (else
        (bind _returnvalue_2 (Actor|GetActorOfClass "/Game/BluePrints/CameraPlayer.CameraPlayer_C"))
        (bind _output_get_2 (Variables|/Game/BluePrints/CameraPlayer.CameraPlayer_C|SetScore _returnvalue_2 (+ (Variables|/Game/BluePrints/CameraPlayer.CameraPlayer_C|GetScore _returnvalue_2) -1)))
        (Development|PrintString (Utilities|String|ToString(Integer) _output_get_2) true true "(R=0.427083,G=0.000000,B=0.010946,A=1.000000)")))
    (Actor|DestroyActor OtherActor)))

(fn ConstructionScript)